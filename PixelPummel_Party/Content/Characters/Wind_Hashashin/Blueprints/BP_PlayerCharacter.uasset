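; Playable 2D flipbook character for a local two-player fighting game, with movement, jump, ground and air attacks, and blocking.
; Enhanced Input drives the character and forwards second-player controls to pawn 1 through Player2 events, with that player's sprite tinted.
; Attacks jump animation nodes behind length-based cooldowns, while hitbox events damage overlapping actors.
; Blocking halves damage, health changes fire a dispatcher, and death disables input before opening the post-game menu.
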(event `Load_Controls`
  (bind _asplayer_controller (cast `PlayerController` (`self.GetController`) :!label _label))
  (bind _returnvalue (pcsubsystem `EnhancedInputLocalPlayerSubsystem` _asplayer_controller))
  (`/Engine/EditorBlueprintResources/StandardMacros.IsValid` _returnvalue
    (:`Is Valid`
      (`EnhancedInputSubsystemInterface.AddMappingContext` _returnvalue "/Game/Controls/IMC_Fighting_Input_Mapping.IMC_Fighting_Input_Mapping" 0 (struct))
      (set `self.playerSpeed` (`CharacterMovementComponent.MaxWalkSpeed` (`self.CharacterMovement`)))
      (set `self.playerMaximumHealth` (`self.playerHealth`)))))

(event `self.ReceiveBeginPlay`
  (goto _label))

(event `EnhancedInput|/Game/Controls/AI_Movement`
  (params (ActionValue :type "Float (double-precision)") (ElapsedSeconds :type "Float (double-precision)") (TriggeredSeconds :type "Float (double-precision)") (InputAction :type "InputAction Object Reference" :default "/Game/Controls/AI_Movement.AI_Movement"))
  ;[1 1 1] "Left" and "Right" movement for the character
  (:`Triggered`
    (`self.AddMovementInput` (1.0 0.0 0.0) ActionValue)))

(event `Player2_Jump`
  ;[1 1 1] "Jumping" movement for the character
  (`self.checkIfBlocking` :!label _label_2
    (:`else`
      _)
    (:`then`
      _))
  (`self.Jump`))

(event `EnhancedInput|/Game/Controls/IA_Jump`
  (params (ActionValue :type Boolean) (ElapsedSeconds :type "Float (double-precision)") (TriggeredSeconds :type "Float (double-precision)") (InputAction :type "InputAction Object Reference" :default "/Game/Controls/IA_Jump.IA_Jump"))
  ;[1 1 1] "Jumping" movement for the character
  (:`Started`
    (goto _label_2))
  (:`Completed`
    (`self.StopJumping`)))

(event `Player2_Attack`
  ;[1 1 1] "Attack" movement for the character
  (`/Engine/EditorBlueprintResources/StandardMacros.DoOnce` false :!label _label_3
    (:`Completed`
      (`self.checkIfBlocking` ; This macro is responsible\nfor checking if the player is \ncurrently blocks. If yes, then \nattack is not possible
        (:`else`
          _)
        (:`then`
          _))
      (set `CharacterMovementComponent.MaxWalkSpeed` 0.0 (`self.CharacterMovement`))
      (if (`NavMovementComponent.IsFalling` (`self.CharacterMovement`))
        ;[1 1 1] "Air attack" movement for the character
        (`PaperZDAnimInstance.JumpToNode` (`PaperZDAnimationComponent.AnimInstance` (`self.AnimationComponent`)) "Air_Attack" "None")
        (`KismetSystemLibrary.Delay` (+ (`PaperFlipbookComponent.GetFlipbookLength` (`self.Sprite`)) 0.7)) ; Responsibe to avoid players spaming attack,\nsince it will wait for the animation to complete.
        (else
          (`PaperZDAnimInstance.JumpToNode` (`PaperZDAnimationComponent.AnimInstance` (`self.AnimationComponent`)) "Attack" "None")
          (`KismetSystemLibrary.Delay` (- (`PaperFlipbookComponent.GetFlipbookLength` (`self.Sprite`)) 0.15)) ; Responsibe to avoid players\nspaming attack,since it will wait\nfor the animation to complete.
        ))
      (set `CharacterMovementComponent.MaxWalkSpeed` (`self.playerSpeed`) (`self.CharacterMovement`))
      (goto _label_3 :!via `Reset`))))

(event `EnhancedInput|/Game/Controls/IA_Attack`
  (params (ActionValue :type Boolean) (ElapsedSeconds :type "Float (double-precision)") (TriggeredSeconds :type "Float (double-precision)") (InputAction :type "InputAction Object Reference" :default "/Game/Controls/IA_Attack.IA_Attack"))
  ;[1 1 1] "Attack" movement for the character
  (:`Started`
    (goto _label_3)))

(event `Player2_Movement`
  (params (axisValue :type "Float (double-precision)"))
  ;[1 1 1] Player2 "left" and "right" movement
  (`self.AddMovementInput` (1.0 0.0 0.0) axisValue))

(event `EnhancedInput|/Game/Controls/IA_Movement_Player2`
  (params (ActionValue :type "Float (double-precision)") (ElapsedSeconds :type "Float (double-precision)") (TriggeredSeconds :type "Float (double-precision)") (InputAction :type "InputAction Object Reference" :default "/Game/Controls/IA_Movement_Player2.IA_Movement_Player2"))
  (bind _player2 (`self.player2`))
  ;[1 1 1] Player2 "left" and "right" movement
  (:`Triggered`
    (`/Engine/EditorBlueprintResources/StandardMacros.IsValid` _player2
      (:`Is Valid`
        (`self.Player2_Movement` _player2 ActionValue))
      (:`Is Not Valid`
        (bind _asbp_player_character (cast `/Game/Characters/Wind_Hashashin/Blueprints/BP_PlayerCharacter` (`GameplayStatics.GetPlayerPawn` 1)))
        (bind _output_get (set `self.player2` _asbp_player_character))
        (`self.Player2_Movement` _output_get ActionValue)))))

(event `Key|W`
  (params (Key :type "Key Structure"))
  (bind _player2 (`self.player2`))
  ;[1 1 1] Player_2 "jump" movement
  (:`Pressed`
    (`/Engine/EditorBlueprintResources/StandardMacros.IsValid` _player2
      (:`Is Valid`
        (`self.Player2_Jump` _player2))
      (:`Is Not Valid`
        (bind _asbp_player_character (cast `/Game/Characters/Wind_Hashashin/Blueprints/BP_PlayerCharacter` (`GameplayStatics.GetPlayerPawn` 1)))
        (bind _output_get (set `self.player2` _asbp_player_character))
        (`self.Player2_Jump` _output_get)))))

(event `Key|LeftMouseButton`
  (params (Key :type "Key Structure"))
  (bind _player2 (`self.player2`))
  ;[1 1 1] Player_2 "attack" movement
  (:`Pressed`
    (`/Engine/EditorBlueprintResources/StandardMacros.IsValid` _player2
      (:`Is Valid`
        (`self.Player2_Attack` _player2))
      (:`Is Not Valid`
        (bind _asbp_player_character (cast `/Game/Characters/Wind_Hashashin/Blueprints/BP_PlayerCharacter` (`GameplayStatics.GetPlayerPawn` 1)))
        (bind _output_get (set `self.player2` _asbp_player_character))
        (`self.Player2_Attack` _output_get)))))

(event `Attack`
  ;[1 1 1] Applies damage to all overlapping characters, except for "self" during "attack"
  (for _array_element (`PrimitiveComponent.GetOverlappingActors` (`self.attack_hitbox`) null)
    (if (!= _array_element self)
      (`GameplayStatics.ApplyDamage` _array_element (`self.Base Damage`)))))

(event `self.ReceiveAnyDamage`
  (params (Damage :type "Float (single-precision)") (DamageType :type "DamageType Object Reference") (InstigatedBy :type "Controller Object Reference") (DamageCauser :type "Actor Object Reference"))
  ;[1 1 1] When damage is applied, if health is 0, then character dies, if not, then the "take-hit" animation executed
  (bind _output_get (set `self.playerHealth` (select `bool` (`self.isBlocking`) :`false` (- (`self.playerHealth`) Damage) :`true` (- (`self.playerHealth`) (/ Damage 2.0))))) ; This node is responsible for\nsetting new players health\nafter the player receives dmg
  (`self.updateHealth`) ; This dispatcher will be\nresponsible for executing event\n(in fighting_level BP), which will\nupdate the players health.
  (if (<= _output_get 0.0)
    (`/Engine/EditorBlueprintResources/StandardMacros.DoOnce` false
      (:`Completed`
        (`PaperZDAnimInstance.JumpToNode` (`PaperZDAnimationComponent.AnimInstance` (`self.AnimationComponent`)) "Death" "None")
        (`self.DisableInput` (`GameplayStatics.GetPlayerPawn` 0) null)
        (`self.DisableInput` (`GameplayStatics.GetPlayerPawn` 1) null)
        (`KismetSystemLibrary.Delay` 3.0)
        (`GameplayStatics.OpenLevelBySoftObjectPtr` "/Game/Menues/PostGameMenue.PostGameMenue")))
    (elif (not (`self.isBlocking`))
      (`PaperZDAnimInstance.JumpToNode` (`PaperZDAnimationComponent.AnimInstance` (`self.AnimationComponent`)) "Damage" "None")
      (set `CharacterMovementComponent.MaxWalkSpeed` 0.0 (`self.CharacterMovement`))
      (`KismetSystemLibrary.RetriggerableDelay` (- (`PaperFlipbookComponent.GetFlipbookLength` (`self.Sprite`)) 0.4))
      (if (not (`self.isBlocking`))
        (set `CharacterMovementComponent.MaxWalkSpeed` (`self.playerSpeed`) (`self.CharacterMovement`))))))

(event `Air_Attack`
  ;[1 1 1] Applies damage to all overlapping characters, except for "self" during "air_attack"
  (for _array_element (`PrimitiveComponent.GetOverlappingActors` (`self.air_attack_hitbox`) null)
    (if (!= _array_element self)
      (`GameplayStatics.ApplyDamage` _array_element (`self.Base Damage`)))))

(event `Player2_Defend`
  ;[1 1 1] "Defend" movement for the character
  (if (not (`NavMovementComponent.IsFalling` (`self.CharacterMovement`))) :!label _label_4
    (set `self.isBlocking` true)
    (set `CharacterMovementComponent.MaxWalkSpeed` 0.0 (`self.CharacterMovement`))))

(event `EnhancedInput|/Game/Controls/IA_Block`
  (params (ActionValue :type Boolean) (ElapsedSeconds :type "Float (double-precision)") (TriggeredSeconds :type "Float (double-precision)") (InputAction :type "InputAction Object Reference" :default "/Game/Controls/IA_Block.IA_Block"))
  ;[1 1 1] "Defend" movement for the character
  (:`Started`
    (goto _label_4))
  (:`Completed`
    (set `self.isBlocking` false :!label _label_5)
    (set `CharacterMovementComponent.MaxWalkSpeed` (`self.playerSpeed`) (`self.CharacterMovement`))))

(event `Player2_Stop_Defending`
  ;[1 1 1] "Defend" movement for the character
  (goto _label_5))

(event `EnhancedInput|/Game/Controls/IA_Block_Player2`
  (params (ActionValue :type Boolean) (ElapsedSeconds :type "Float (double-precision)") (TriggeredSeconds :type "Float (double-precision)") (InputAction :type "InputAction Object Reference" :default "/Game/Controls/IA_Block_Player2.IA_Block_Player2"))
  ;[1 1 1] "Defend" movement for Player2
  (:`Started`
    (`/Engine/EditorBlueprintResources/StandardMacros.IsValid` (`self.player2`)
      (:`Is Valid`
        (`self.Player2_Defend` (`self.player2`)))
      (:`Is Not Valid`
        (bind _asbp_player_character (cast `/Game/Characters/Wind_Hashashin/Blueprints/BP_PlayerCharacter` (`GameplayStatics.GetPlayerPawn` 1)))
        (bind _output_get (set `self.player2` _asbp_player_character))
        (`self.Player2_Defend` _output_get))))
  (:`Completed`
    (`/Engine/EditorBlueprintResources/StandardMacros.IsValid` (`self.player2`)
      (:`Is Valid`
        (`self.Player2_Stop_Defending` (`self.player2`)))
      (:`Is Not Valid`
        (bind _asbp_player_character_2 (cast `/Game/Characters/Wind_Hashashin/Blueprints/BP_PlayerCharacter` (`GameplayStatics.GetPlayerPawn` 1)))
        (bind _output_get_2 (set `self.player2` _asbp_player_character_2))
        (`self.Player2_Stop_Defending` _output_get_2)))))

(fn `UserConstructionScript`
  (if (`self.isPlayer2`)
    (`PaperFlipbookComponent.SetSpriteColor` (`self.Sprite`) (struct :`R` 0.274638 :`G` 0.335803 :`B` 1.0 :`A` 1.0))))